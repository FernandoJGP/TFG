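; PowerUp is a pickup that sets IsPowered on the player's MainCharacter and plays a sound when the player overlaps it.
; Collecting one disables every PowerUp in the level, and each also disables itself at BeginPlay if the player is already powered.
; Enable and Disable swap the sphere's material, toggle collection and start or stop the floating audio.
; A looping MoveComponentTo and Delay chain bobs the sphere continuously, even while disabled.
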(event `self.ReceiveBeginPlay`
  (set `self.BallRelativeLocation` (`SceneComponent.RelativeLocation` (`self.GoldSphere`)))
  (`AudioComponent.Play` (`self.Floating`) 0.0)
  (`self.Move`)
  (bind _asmain_character (cast `MainCharacter` (`GameplayStatics.GetPlayerPawn` 0)))
  (if (`MainCharacter.bIsPowered` _asmain_character)
    (`self.Disable`)))

(event `self.ReceiveActorBeginOverlap`
  (params (OtherActor :type "Actor Object Reference"))
  (if (`self.IsEnable`)
    (if (== OtherActor (`GameplayStatics.GetPlayerPawn` 0))
      (bind _asmain_character (cast `MainCharacter` (`GameplayStatics.GetPlayerPawn` 0)))
      (set `MainCharacter.bIsPowered` true _asmain_character)
      (`GameplayStatics.PlaySoundAtLocation` "/Game/SFX/PowerUp.PowerUp" (`self.K2_GetActorLocation`))
      (bind _outactors (`GameplayStatics.GetAllActorsOfClass` "PowerUp_C"))
      (for _array_element _outactors
        (`self.Disable` _array_element)))))

(event `Enable`
  (`PrimitiveComponent.SetMaterial` (`self.GoldSphere`) 0 "/Game/Blueprints/LevelPuzzles/Materials/MetalicGold.MetalicGold")
  (set `self.IsEnable` true)
  (`AudioComponent.Play` (`self.Floating`) 0.0))

(event `Disable`
  (`PrimitiveComponent.SetMaterial` (`self.GoldSphere`) 0 "/Game/Blueprints/LevelPuzzles/Materials/Reflaction.Reflaction")
  (set `self.IsEnable` false)
  (`AudioComponent.Stop` (`self.Floating`)))

(event `Move`
  (`KismetSystemLibrary.MoveComponentTo` (`self.GoldSphere`) (+ (`self.BallRelativeLocation`) (0.0 0.0 10.0)) (struct) false false (`self.TimeToReachLocation`) :!label _label)
  (`KismetSystemLibrary.Delay` (`self.DelayBetweenToggles`))
  (`KismetSystemLibrary.MoveComponentTo` (`self.GoldSphere`) (`self.BallRelativeLocation`) (struct) false false (`self.TimeToReachLocation`))
  (`KismetSystemLibrary.Delay` (`self.DelayBetweenToggles`))
  (goto _label))

(fn `UserConstructionScript`
  (`AudioComponent.SetSound` (`self.Floating`) "/Game/SFX/Floating.Floating")
  (`AudioComponent.AdjustAttenuation` (`self.Floating`) (make `SoundAttenuationSettings` true true false false false false 0.0 0.0 "SPATIALIZATION_Default" null 3000.0 6000.0 20000.0 20000.0 30.0 60.0 1.0 1.0 1.0 1.0 1.0 1.0 "ECC_Visibility" 20000.0 1.0 0.1 null null 0.3 0.95 400.0 4000.0 "NaturalSound")))