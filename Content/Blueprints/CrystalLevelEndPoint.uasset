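; A floating crystal that marks a level's end and sends the player on to the next level.
; Overlap enables input and opens a gate, so pressing Action while facing the crystal within 30 degrees triggers the exit.
; The exit writes a fresh next-level start to the MainSaveGame slot, disables player input, plays thunder and a fade-to-white sequence, then opens that level.
; BeginPlay loops MoveComponentTo to bob and turn the mesh.
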(event `InputAction|Action`
  (params (Key :type "Key Structure" :default "AnyKey"))
  (bind _returnvalue (`GameplayStatics.GetPlayerPawn` 0))
  (bind _returnvalue_2 (`GameplayStatics.GetPlayerPawn` 0))
  (:`Pressed`
    (`/Engine/EditorBlueprintResources/StandardMacros.Gate` true :!label _label
      (:`Exit`
        (if (`KismetMathLibrary.InRange_FloatFloat` (`KismetMathLibrary.DegAcos` (`KismetMathLibrary.Dot_VectorVector` (`KismetMathLibrary.Normal` (`self.GetActorForwardVector` _returnvalue)) (`KismetMathLibrary.Normal` (`KismetMathLibrary.MakeVector` (- (.x (`self.K2_GetActorLocation`)) (.x (`self.K2_GetActorLocation` _returnvalue))) (- (.y (`self.K2_GetActorLocation`)) (.y (`self.K2_GetActorLocation` _returnvalue))))))) -30.0 30.0)
          (bind _returnvalue_3 (`GameplayStatics.DoesSaveGameExist` (`self.SaveSlotName`)))
          (if _returnvalue_3
            (bind _returnvalue_4 (`GameplayStatics.LoadGameFromSlot` (`self.SaveSlotName`)))
            (set `self.SaveReference` _returnvalue_4)
            (else
              (bind _returnvalue_5 (`GameplayStatics.CreateSaveGameObject` "/Game/Blueprints/SaveGames/MainSaveGame.MainSaveGame_C"))
              (set `self.SaveReference` _returnvalue_5)))
          (bind _asmain_save_game (cast `/Game/Blueprints/SaveGames/MainSaveGame` (`self.SaveReference`)))
          (set `/Game/Blueprints/SaveGames/MainSaveGame.Level` (`self.NextLevel`) _asmain_save_game)
          (set `/Game/Blueprints/SaveGames/MainSaveGame.Location` (0.0 0.0 0.0) _asmain_save_game)
          (set `/Game/Blueprints/SaveGames/MainSaveGame.Rotation` (struct) _asmain_save_game)
          (set `/Game/Blueprints/SaveGames/MainSaveGame.bFromStart` true _asmain_save_game)
          (set `/Game/Blueprints/SaveGames/MainSaveGame.bIsPowered` false _asmain_save_game)
          (`GameplayStatics.SaveGameToSlot` (`self.SaveReference`) (`self.SaveSlotName`))
          (`self.DisableInput` _returnvalue_2 (`GameplayStatics.GetPlayerController` 0))
          (`GameplayStatics.PlaySoundAtLocation` "/Game/SFX/Thunder.Thunder" (`self.K2_GetActorLocation` _returnvalue_2))
          (bind (_outactor _returnvalue_6) (`LevelSequencePlayer.CreateLevelSequencePlayer` "/Game/Sequences/FadeToWhite.FadeToWhite"))
          (`MovieSceneSequencePlayer.Play` _returnvalue_6)
          (`KismetSystemLibrary.Delay` (`MovieSceneSequencePlayer.GetLength` _returnvalue_6))
          (`GameplayStatics.OpenLevel` (`self.NextLevel`)))))))

(event `self.ReceiveActorBeginOverlap`
  (params (OtherActor :type "Actor Object Reference"))
  (if (== OtherActor (`GameplayStatics.GetPlayerPawn` 0))
    (`self.EnableInput` (`GameplayStatics.GetPlayerController` 0))
    (goto _label :!via `Open`)))

(event `self.ReceiveActorEndOverlap`
  (params (OtherActor :type "Actor Object Reference"))
  (if (== OtherActor (`GameplayStatics.GetPlayerPawn` 0))
    (`self.DisableInput` (`GameplayStatics.GetPlayerController` 0))
    (goto _label :!via `Close`)))

(event `self.ReceiveBeginPlay`
  (`KismetSystemLibrary.MoveComponentTo` (`self.CrystalMesh`) (0.0 0.0 100.0) (struct :`Yaw` 180.0) false false 2.5 :!label _label_2)
  (`KismetSystemLibrary.MoveComponentTo` (`self.CrystalMesh`) (0.0 0.0 50.0) (struct) false false 2.5)
  (goto _label_2))

(fn `UserConstructionScript`)