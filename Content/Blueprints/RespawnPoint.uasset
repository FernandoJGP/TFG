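; Respawn checkpoint actor that saves the current level and a spawn transform whenever an actor overlaps it, with no filter on which actor.
; It prints a "Saving" message in English or Spanish, based on the language in the settings save.
; It then loads or creates the MainSaveGame, stores a height-offset location and Arrow-facing rotation, clears FromStart, and writes the slot.
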(event `self.ReceiveActorBeginOverlap`
  (params (OtherActor :type "Actor Object Reference"))
  (bind _returnvalue (`SceneComponent.K2_GetComponentLocation` (`self.DefaultSceneRoot`)))
  (bind _returnvalue_2 (`GameplayStatics.DoesSaveGameExist` (`self.SettingsSlotName`)))
  (if _returnvalue_2
    (bind _returnvalue_3 (`GameplayStatics.LoadGameFromSlot` (`self.SettingsSlotName`)))
    (bind _assettings_save_game (cast `/Game/Blueprints/SaveGames/SettingsSaveGame` _returnvalue_3))
    (switch `string` (`/Game/Blueprints/SaveGames/SettingsSaveGame.Language` _assettings_save_game)
      (:`Default`
        (set `self.SavingText` "Saving..." :!label _label))
      (:`en`
        (goto _label))
      (:`es`
        (set `self.SavingText` "Guardando...")))
    (else
      (set `self.SavingText` "Saving...")))
  (`KismetSystemLibrary.PrintString` (`KismetTextLibrary.Conv_TextToString` (`self.SavingText`)) true true (struct :`R` 0.06492 :`B` 1.0 :`A` 1.0) 2.0)
  (bind _returnvalue_4 (`GameplayStatics.DoesSaveGameExist` (`self.SaveSlotName`)))
  (if _returnvalue_4
    (bind _returnvalue_5 (`GameplayStatics.LoadGameFromSlot` (`self.SaveSlotName`)))
    (set `self.SaveReference` _returnvalue_5)
    (else
      (bind _returnvalue_6 (`GameplayStatics.CreateSaveGameObject` "/Game/Blueprints/SaveGames/MainSaveGame.MainSaveGame_C"))
      (set `self.SaveReference` _returnvalue_6)))
  (bind _asmain_save_game (cast `/Game/Blueprints/SaveGames/MainSaveGame` (`self.SaveReference`)))
  (bind _returnvalue_7 (`GameplayStatics.GetCurrentLevelName` true))
  (set `/Game/Blueprints/SaveGames/MainSaveGame.Level` (`KismetStringLibrary.Conv_StringToName` _returnvalue_7) _asmain_save_game)
  (set `/Game/Blueprints/SaveGames/MainSaveGame.Location` (+ (`SceneComponent.K2_GetComponentLocation` (`self.DefaultSceneRoot`)) (0.0 0.0 100.0)) _asmain_save_game)
  (set `/Game/Blueprints/SaveGames/MainSaveGame.Rotation` (`KismetMathLibrary.RInterpTo` (`SceneComponent.K2_GetComponentRotation` (`self.DefaultSceneRoot`)) (`KismetMathLibrary.FindLookAtRotation` _returnvalue (+ _returnvalue (`SceneComponent.GetForwardVector` (`self.Arrow`))))) _asmain_save_game)
  (set `/Game/Blueprints/SaveGames/MainSaveGame.bFromStart` false _asmain_save_game)
  (`GameplayStatics.SaveGameToSlot` (`self.SaveReference`) (`self.SaveSlotName`)))

(fn `UserConstructionScript`)