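; PowerDown is a portal trigger that strips the player's power and returns pickups to where they started.
; On BeginPlay it gives the Portal a dynamic material with a lowered Efficiency parameter.
; Player overlap clears IsPowered, plays a sound, re-enables every PowerUp, and detaches and resets all "pickup"-tagged Pickables.
; A tagged Pickable entering alone gets the same reset without detaching, with physics disabled around the teleport to its initial transform.
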(event `self.ReceiveBeginPlay`
  (bind _portal (`self.Portal`))
  (bind _asprimitive_component (cast `PrimitiveComponent` _portal))
  (bind _returnvalue (`PrimitiveComponent.CreateDynamicMaterialInstance` _asprimitive_component 0 (`PrimitiveComponent.GetMaterial` _portal 0)))
  (`MaterialInstanceDynamic.SetScalarParameterValue` _returnvalue "Efficiency" 0.25))

(event `self.ReceiveActorBeginOverlap`
  (params (OtherActor :type "Actor Object Reference"))
  (bind _returnvalue (`GameplayStatics.GetPlayerPawn` 0))
  (if (== OtherActor _returnvalue)
    (bind _asmain_character (cast `MainCharacter` _returnvalue))
    (set `MainCharacter.bIsPowered` false _asmain_character)
    (`GameplayStatics.PlaySoundAtLocation` "/Game/SFX/PowerDown.PowerDown" (`self.K2_GetActorLocation`))
    (bind _outactors (`GameplayStatics.GetAllActorsOfClass` "/Game/Blueprints/PowerUp.PowerUp_C"))
    (for _array_element _outactors
      (`/Game/Blueprints/PowerUp.Enable` _array_element))
    (bind _outactors_2 (`GameplayStatics.GetAllActorsOfClass` "/Game/Blueprints/LevelPuzzles/Pickable.Pickable_C"))
    (for _array_element_2 _outactors_2
      (if (`self.ActorHasTag` _array_element_2 "pickup")
        (`self.K2_DetachFromActor` _array_element_2 "KeepRelative" "KeepRelative" "KeepRelative")
        (bind _aspickable (cast `/Game/Blueprints/LevelPuzzles/Pickable` _array_element_2))
        (`/Game/Blueprints/LevelPuzzles/Pickable.DisablePhysics` _aspickable)
        (`self.K2_SetActorLocationAndRotation` _aspickable (`/Game/Blueprints/LevelPuzzles/Pickable.InitialWorldPosition` _aspickable) (`/Game/Blueprints/LevelPuzzles/Pickable.InitialWorldRotation` _aspickable) false false)
        (set `/Game/Blueprints/LevelPuzzles/Pickable.IsBusy` true _aspickable)
        (set `/Game/Blueprints/LevelPuzzles/Pickable.IsPicked` false _aspickable)
        (`/Game/Blueprints/LevelPuzzles/Pickable.EnablePhysics` _aspickable)
        (set `/Game/Blueprints/LevelPuzzles/Pickable.IsBusy` false _aspickable)))
    (elif (`self.ActorHasTag` OtherActor "pickup")
      (bind _aspickable_2 (cast `/Game/Blueprints/LevelPuzzles/Pickable` OtherActor))
      (`/Game/Blueprints/LevelPuzzles/Pickable.DisablePhysics` _aspickable_2)
      (`self.K2_SetActorLocationAndRotation` _aspickable_2 (`/Game/Blueprints/LevelPuzzles/Pickable.InitialWorldPosition` _aspickable_2) (`/Game/Blueprints/LevelPuzzles/Pickable.InitialWorldRotation` _aspickable_2) false false)
      (set `/Game/Blueprints/LevelPuzzles/Pickable.IsBusy` true _aspickable_2)
      (set `/Game/Blueprints/LevelPuzzles/Pickable.IsPicked` false _aspickable_2)
      (`/Game/Blueprints/LevelPuzzles/Pickable.EnablePhysics` _aspickable_2)
      (set `/Game/Blueprints/LevelPuzzles/Pickable.IsBusy` false _aspickable_2))))

(fn `UserConstructionScript`)