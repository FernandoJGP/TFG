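; LevelEndPoint is an end-of-level trigger that saves progression and opens the next level when any actor overlaps it.
; On overlap it loads the save slot, or creates a MainSaveGame if none exists.
; It writes NextLevel into the save, zeroes the stored location and rotation, and sets FromStart.
; It then saves to the slot and opens NextLevel by name, without filtering the overlapping actor.
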(event `self.ReceiveActorBeginOverlap`
  (params (OtherActor :type "Actor Object Reference"))
  (bind _returnvalue (`GameplayStatics.DoesSaveGameExist` (`self.SaveSlotName`)))
  (if _returnvalue
    (bind _returnvalue_2 (`GameplayStatics.LoadGameFromSlot` (`self.SaveSlotName`)))
    (set `self.SaveReference` _returnvalue_2)
    (else
      (bind _returnvalue_3 (`GameplayStatics.CreateSaveGameObject` "/Game/Blueprints/SaveGames/MainSaveGame.MainSaveGame_C"))
      (set `self.SaveReference` _returnvalue_3)))
  (bind _asmain_save_game (cast `/Game/Blueprints/SaveGames/MainSaveGame` (`self.SaveReference`)))
  (set `/Game/Blueprints/SaveGames/MainSaveGame.Level` (`self.NextLevel`) _asmain_save_game)
  (set `/Game/Blueprints/SaveGames/MainSaveGame.Location` (0.0 0.0 0.0) _asmain_save_game)
  (set `/Game/Blueprints/SaveGames/MainSaveGame.Rotation` (struct) _asmain_save_game)
  (set `/Game/Blueprints/SaveGames/MainSaveGame.bFromStart` true _asmain_save_game)
  (`GameplayStatics.SaveGameToSlot` (`self.SaveReference`) (`self.SaveSlotName`))
  (`GameplayStatics.OpenLevel` (`self.NextLevel`)))

(fn `UserConstructionScript`)