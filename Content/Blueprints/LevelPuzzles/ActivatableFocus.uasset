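; ActivatableFocus is a level-puzzle Blueprint that shows its enabled or disabled state through the color of a spotlight.
; It overrides the Enable and Disable events, calls the parent behavior, then sets the SpotLight to EnabledLightColor or DisabledLightColor.
; BeginPlay is an unused stub and the construction script only calls its parent.
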(event `self.Enable`
  (`parent.Enable`)
  (`LightComponent.SetLightColor` (`self.SpotLight`) (`self.EnabledLightColor`) true))

(event `self.Disable`
  (`parent.Disable`)
  (`LightComponent.SetLightColor` (`self.SpotLight`) (`self.DisabledLightColor`) true))

(fn `UserConstructionScript`
  (`parent.UserConstructionScript`))