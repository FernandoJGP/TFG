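; Pressure plate puzzle switch that lowers and enables its linked Activatables when the player steps on it or enough weight rests on it.
; With a weight objective, the player's fixed weight and tagged Pickable weights feed a display and threshold check.
; Activation also requires any listed prerequisite powerables to be active.
; Release plays a ticking delay before disabling targets, and the trigger box grows taller while the player overlaps it.
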(event `self.ReceiveActorBeginOverlap`
  (params (OtherActor :type "Actor Object Reference"))
  (if (== OtherActor (`GameplayStatics.GetPlayerPawn` 0))
    (`BoxComponent.SetBoxExtent` (`self.Box`) (36.0 36.0 70.0) true)
    (if (> (`self.WeightObjective`) 0.0)
      (set `self.WeightCurrent` (+ (`self.WeightCurrent`) 80.0))
      (`self.UpdateDisplay` :!label _label)
      (if (>= (`self.WeightCurrent`) (`self.WeightObjective`))
        (if (not (`self.IsActivated`)) :!label _label_2
          (if (> (`KismetArrayLibrary.Array_Length` (`self.OtherPowerablesNeeded`)) 0)
            (set `self.AllNeededsAreActivated` true)
            (for _array_element (`self.OtherPowerablesNeeded`)
              (if (not (`/Game/Blueprints/LevelPuzzles/Powerable.IsActivated` _array_element))
                (set `self.AllNeededsAreActivated` false)))
            (if (`self.AllNeededsAreActivated`)
              (`GameplayStatics.PlaySoundAtLocation` "/Game/SFX/Switch.Switch" (`self.K2_GetActorLocation`) :!label _label_3)
              (`KismetSystemLibrary.MoveComponentTo` (`self.PressurePlate`) (0.0 0.0 -3.5) (struct) true true)
              (for _array_element_2 (`self.Activatables`)
                (if (not (`/Game/Blueprints/LevelPuzzles/Activatable.IsEnable` _array_element_2))
                  (`/Game/Blueprints/LevelPuzzles/Activatable.Enable` _array_element_2)))
              (set `self.IsActivated` true))
            (else
              (goto _label_3)))))
      (else
        (goto _label_2)))
    (elif (`self.ActorHasTag` OtherActor "pickup")
      (if (> (`self.WeightObjective`) 0.0)
        (bind _aspickable (cast `/Game/Blueprints/LevelPuzzles/Pickable` OtherActor))
        (set `self.WeightCurrent` (+ (`self.WeightCurrent`) (`/Game/Blueprints/LevelPuzzles/Pickable.Weight` _aspickable)))
        (goto _label)))))

(event `self.ReceiveActorEndOverlap`
  (params (OtherActor :type "Actor Object Reference"))
  (if (== OtherActor (`GameplayStatics.GetPlayerPawn` 0))
    (`BoxComponent.SetBoxExtent` (`self.Box`) (36.0 36.0 10.0) true)
    (if (> (`self.WeightObjective`) 0.0)
      (set `self.WeightCurrent` (- (`self.WeightCurrent`) 80.0))
      (`self.UpdateDisplay` :!label _label_4)
      (if (< (`self.WeightCurrent`) (`self.WeightObjective`))
        (if (`self.IsActivated`) :!label _label_5
          (`AudioComponent.Play` (`self.ClockAudio`) 0.0)
          (`KismetSystemLibrary.Delay` (`self.TimeToToggle`))
          (if (`AudioComponent.IsPlaying` (`self.ClockAudio`))
            (`AudioComponent.Stop` (`self.ClockAudio`))
            (if (or (<= (`self.WeightObjective`) 0.0) (< (`self.WeightCurrent`) (`self.WeightObjective`)))
              (`GameplayStatics.PlaySoundAtLocation` "/Game/SFX/Switch.Switch" (`self.K2_GetActorLocation`))
              (`KismetSystemLibrary.MoveComponentTo` (`self.PressurePlate`) (0.0 0.0 3.5) (struct) true true :!label _label_6)
              (for _array_element (`self.Activatables`)
                (`/Game/Blueprints/LevelPuzzles/Activatable.Disable` _array_element))
              (set `self.IsActivated` false)))
          (else
            (goto _label_6))))
      (else
        (goto _label_5)))
    (elif (`self.ActorHasTag` OtherActor "pickup")
      (if (> (`self.WeightObjective`) 0.0)
        (bind _aspickable (cast `/Game/Blueprints/LevelPuzzles/Pickable` OtherActor))
        (set `self.WeightCurrent` (- (`self.WeightCurrent`) (`/Game/Blueprints/LevelPuzzles/Pickable.Weight` _aspickable)))
        (goto _label_4)))))

(event `UpdateDisplay`
  (if (> (`self.WeightObjective`) 0.0)
    (set `/Game/Blueprints/LevelPuzzles/DigitalDisplayObjective.Current` (`self.WeightCurrent`) (`self.Display`))
    (`/Game/Blueprints/LevelPuzzles/DigitalDisplayObjective.UpdateText` (`self.Display`))))

(event `self.ReceiveBeginPlay`
  (`self.UpdateDisplay`))

(fn `AllNeededsActivated`
  (returns (AllActivated :type Boolean))
  (if (> (`KismetArrayLibrary.Array_Length` (`self.OtherPowerablesNeeded`)) 0)
    (for _array_element _
      (if (not (`/Game/Blueprints/LevelPuzzles/Powerable.IsActivated` _array_element))
        (return false)))
    (return true)
    (else
      (return false))))

(fn `UserConstructionScript`
  (`AudioComponent.SetSound` (`self.ClockAudio`) "/Game/SFX/ClockTicking.ClockTicking")
  (if (> (`self.WeightObjective`) 0.0)
    (set `/Game/Blueprints/LevelPuzzles/DigitalDisplayObjective.Current` (`self.WeightCurrent`) (`self.Display`))
    (set `/Game/Blueprints/LevelPuzzles/DigitalDisplayObjective.Objective` (`self.WeightObjective`) (`self.Display`))
    (`/Game/Blueprints/LevelPuzzles/DigitalDisplayObjective.UpdateText` (`self.Display`))))