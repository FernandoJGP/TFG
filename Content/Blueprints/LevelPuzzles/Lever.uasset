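; A puzzle lever the player flips with the Action input while inside its overlap area and facing it within 30 degrees.
; Toggling animates the handle, plays a switch sound and enables or disables linked Activatables, which also require all OtherPowerablesNeeded to be active, and ActivatablesAlways, which follow this lever alone.
; An optional TimeToToggle plays a ticking clock, blocks further use and flips the lever back when it expires.
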(event `self.ReceiveBeginPlay`
  (`self.UpdateLeverHander`))

(event `InputAction|Action`
  (params (Key :type "Key Structure" :default "AnyKey"))
  (bind _returnvalue (`GameplayStatics.GetPlayerPawn` 0))
  (:`Pressed`
    (`/Engine/EditorBlueprintResources/StandardMacros.Gate` true :!label _label
      (:`Exit`
        (if (and (not (`self.IsBusy`)) (`KismetMathLibrary.InRange_FloatFloat` (`KismetMathLibrary.DegAcos` (`KismetMathLibrary.Dot_VectorVector` (`KismetMathLibrary.Normal` (`self.GetActorForwardVector` _returnvalue)) (`KismetMathLibrary.Normal` (`KismetMathLibrary.MakeVector` (- (.x (`self.K2_GetActorLocation`)) (.x (`self.K2_GetActorLocation` _returnvalue))) (- (.y (`self.K2_GetActorLocation`)) (.y (`self.K2_GetActorLocation` _returnvalue))))))) -30.0 30.0))
          (set `self.IsBusy` true)
          (`self.ToggleActive`)
          (if (> (`self.TimeToToggle`) 0.0)
            (`AudioComponent.Play` (`self.ClockAudio`) 0.0)
            (`KismetSystemLibrary.Delay` (`self.TimeToToggle`))
            (`self.ToggleActive`)
            (set `self.IsBusy` false)
            (if (`AudioComponent.IsPlaying` (`self.ClockAudio`))
              (`AudioComponent.Stop` (`self.ClockAudio`)))
            (else
              (set `self.IsBusy` false))))))))

(event `self.ReceiveActorBeginOverlap`
  (params (OtherActor :type "Actor Object Reference"))
  (if (== OtherActor (`GameplayStatics.GetPlayerPawn` 0))
    (`self.EnableInput` (`GameplayStatics.GetPlayerController` 0))
    (goto _label :!via `Open`)))

(event `self.ReceiveActorEndOverlap`
  (params (OtherActor :type "Actor Object Reference"))
  (if (== OtherActor (`GameplayStatics.GetPlayerPawn` 0))
    (`self.DisableInput` (`GameplayStatics.GetPlayerController` 0))
    (goto _label :!via `Close`)))

(event `UpdateLeverHander`
  (if (`self.IsActivated`)
    (`KismetSystemLibrary.MoveComponentTo` (`self.LeverHanderRoot`) (`SceneComponent.RelativeLocation` (`self.LeverHanderRoot`)) (`KismetMathLibrary.MakeRotator` 90.0) true true)
    (else
      (`KismetSystemLibrary.MoveComponentTo` (`self.LeverHanderRoot`) (`SceneComponent.RelativeLocation` (`self.LeverHanderRoot`)) (`KismetMathLibrary.MakeRotator` 0.0) true true))))

(event `ToggleActive`
  (set `self.IsActivated` (not (`self.IsActivated`)))
  (`self.UpdateLeverHander`)
  (`GameplayStatics.PlaySoundAtLocation` "/Game/SFX/Switch.Switch" (`self.K2_GetActorLocation`))
  (set `self.AllNeededsAreActivated` true)
  (if (> (`KismetArrayLibrary.Array_Length` (`self.OtherPowerablesNeeded`)) 0)
    (for _array_element (`self.OtherPowerablesNeeded`)
      (if (not (`/Game/Blueprints/LevelPuzzles/Powerable.IsActivated` _array_element))
        (set `self.AllNeededsAreActivated` false))))
  (`|ExecutionSequence`
    (:`then_0`
      (if (and (`self.IsActivated`) (`self.AllNeededsAreActivated`))
        (for _array_element_2 (`self.Activatables`)
          (`/Game/Blueprints/LevelPuzzles/Activatable.Enable` _array_element_2))
        (else
          (for _array_element_3 (`self.Activatables`)
            (`/Game/Blueprints/LevelPuzzles/Activatable.Disable` _array_element_3)))))
    (:`then_1`
      (if (`self.IsActivated`)
        (for _array_element_4 (`self.ActivatablesAlways`)
          (`/Game/Blueprints/LevelPuzzles/Activatable.Enable` _array_element_4))
        (else
          (for _array_element_5 (`self.ActivatablesAlways`)
            (`/Game/Blueprints/LevelPuzzles/Activatable.Disable` _array_element_5)))))))

(fn `UserConstructionScript`
  (`AudioComponent.SetSound` (`self.ClockAudio`) "/Game/SFX/ClockTicking.ClockTicking"))