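; Puzzle sliding door with two panels that open on Enable and close on Disable, extending a parent's enable/disable logic.
; BeginPlay caches each panel's starting relative location and the location of its destination component.
; Both events move the panels between these locations with eased MoveComponentTo over a shared OpenDelay.
; Open and close sounds play only when IsEnable is true, at a Volume that each event then sets to full.
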(event `self.ReceiveBeginPlay`
  (set `self.LeftDoorStartingLocation` (`SceneComponent.RelativeLocation` (`self.Left Door`)))
  (set `self.RightDoorStartingLocation` (`SceneComponent.RelativeLocation` (`self.Right Door`)))
  (set `self.LeftDoorDestinationLocation` (`SceneComponent.RelativeLocation` (`self.Left Door Destination`)))
  (set `self.RightDoorDestinationLocation` (`SceneComponent.RelativeLocation` (`self.Right Door Destination`)))
  (`parent.ReceiveBeginPlay`))

(event `self.Enable`
  (`parent.Enable`)
  (if (`self.IsEnable`)
    (`GameplayStatics.PlaySoundAtLocation` "/Game/SFX/DoorOpen.DoorOpen" (`self.K2_GetActorLocation`) (struct) (`self.Volume`) 1.0 0.0 "/Game/SFX/NaturalSoundAttenuation.NaturalSoundAttenuation"))
  (`|ExecutionSequence`
    (:`then_0`
      (`KismetSystemLibrary.MoveComponentTo` (`self.Left Door`) (`self.LeftDoorDestinationLocation`) (struct) true true (`self.OpenDelay`)))
    (:`then_1`
      (`KismetSystemLibrary.MoveComponentTo` (`self.Right Door`) (`self.RightDoorDestinationLocation`) (struct) true true (`self.OpenDelay`))
      (set `self.Volume` 1.0))))

(event `self.Disable`
  (`parent.Disable`)
  (if (`self.IsEnable`)
    (`GameplayStatics.PlaySoundAtLocation` "/Game/SFX/DoorClose.DoorClose" (`self.K2_GetActorLocation`) (struct) (`self.Volume`) 1.0 0.0 "/Game/SFX/NaturalSoundAttenuation.NaturalSoundAttenuation"))
  (`|ExecutionSequence`
    (:`then_0`
      (`KismetSystemLibrary.MoveComponentTo` (`self.Left Door`) (`self.LeftDoorStartingLocation`) (struct) true true (`self.OpenDelay`)))
    (:`then_1`
      (`KismetSystemLibrary.MoveComponentTo` (`self.Right Door`) (`self.RightDoorStartingLocation`) (struct) true true (`self.OpenDelay`))
      (set `self.Volume` 1.0))))

(fn `UserConstructionScript`)