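; Elevator level-puzzle Blueprint that moves its Floor component and is activated by a Lever child actor.
; On BeginPlay it registers itself as the only entry in the lever's Activatables list.
; The construction script sets Floor as the ObjectToMove, while Enable and Disable defer entirely to the parent class, which presumably handles the movement.
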(event `self.ReceiveBeginPlay`
  (`parent.ReceiveBeginPlay`)
  (bind _aslever (cast `/Game/Blueprints/LevelPuzzles/Lever` (`ChildActorComponent.ChildActor` (`self.Lever`))))
  (set `/Game/Blueprints/LevelPuzzles/Powerable.Activatables` (`|MakeArray` self :!type "/Game/Blueprints/LevelPuzzles/Activatable Object Reference") _aslever))

(event `/Game/Blueprints/LevelPuzzles/Activatable.Enable`
  (`parent.Enable`))

(event `/Game/Blueprints/LevelPuzzles/Activatable.Disable`
  (`parent.Disable`))

(fn `UserConstructionScript`
  (`parent.UserConstructionScript`)
  (set `self.ObjectToMove` (`self.Floor`)))