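; Puzzle block child Blueprint that adds configurable top, bottom, X and Y spikes, each a mesh paired with an overlap box.
; The construction script sets spike visibility and overlap events from per-side flags and IsEnable.
; Enable and Disable toggle them only when HideSpikesIfDisabled is set, and Disable can be locked out after a first enable.
; Each toggle, including construction, plays a sword-swipe sound, then sets its volume to full.
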(event `self.ReceiveBeginPlay`
  (`parent.ReceiveBeginPlay`))

(event `self.Enable`
  (bind _topspikes (`self.TopSpikes`))
  (bind _bottomspikes (`self.BottomSpikes`))
  (bind _x_spikes (`self.X+Spikes`))
  (bind _x_spikes_2 (`self.X-Spikes`))
  (bind _y_spikes (`self.Y+Spikes`))
  (bind _y_spikes_2 (`self.Y-Spikes`))
  (`parent.Enable`)
  (if (`self.HideSpikesIfDisabled`)
    (`|ExecutionSequence`
      (:`then_0`
        (`SceneComponent.SetVisibility` (`self.TopSpikesMesh`) _topspikes true)
        (set `PrimitiveComponent.bGenerateOverlapEvents` _topspikes (`self.TopSpikesCollisionBox`)))
      (:`then_1`
        (`SceneComponent.SetVisibility` (`self.BottomSpikesMesh`) _bottomspikes true)
        (set `PrimitiveComponent.bGenerateOverlapEvents` _bottomspikes (`self.BottomSpikesCollisionBox`)))
      (:`then_2`
        (`SceneComponent.SetVisibility` (`self.X+SpikesMesh`) _x_spikes true)
        (set `PrimitiveComponent.bGenerateOverlapEvents` _x_spikes (`self.X+SpikesCollisionBox`)))
      (:`then_3`
        (`SceneComponent.SetVisibility` (`self.X-SpikesMesh`) _x_spikes_2 true)
        (set `PrimitiveComponent.bGenerateOverlapEvents` _x_spikes_2 (`self.X-SpikesCollisionBox`)))
      (:`then_4`
        (`SceneComponent.SetVisibility` (`self.Y+SpikesMesh`) _y_spikes true)
        (set `PrimitiveComponent.bGenerateOverlapEvents` _y_spikes (`self.Y+SpikesCollisionBox`)))
      (:`then_5`
        (`SceneComponent.SetVisibility` (`self.Y-SpikesMesh`) _y_spikes_2 true)
        (set `PrimitiveComponent.bGenerateOverlapEvents` _y_spikes_2 (`self.Y-SpikesCollisionBox`)))
      (:`then_6`
        (`GameplayStatics.PlaySoundAtLocation` "/Game/SFX/SwordSwipe.SwordSwipe" (`self.K2_GetActorLocation`) (struct) (`self.SwordSwipeVolume`) 1.0 0.0 "/Game/SFX/NaturalSoundAttenuation.NaturalSoundAttenuation" "/Game/Music/StandardSoundConcurrency.StandardSoundConcurrency")
        (set `self.SwordSwipeVolume` 1.0)))))

(event `self.Disable`
  (`parent.Disable`)
  (if (or (not (`self.WasEnableAtLeastOneTime`)) (`self.CanBeDisabledAfterEnabled`))
    (if (`self.HideSpikesIfDisabled`)
      (`|ExecutionSequence`
        (:`then_0`
          (`SceneComponent.SetVisibility` (`self.TopSpikesMesh`) false true)
          (set `PrimitiveComponent.bGenerateOverlapEvents` false (`self.TopSpikesCollisionBox`)))
        (:`then_1`
          (`SceneComponent.SetVisibility` (`self.BottomSpikesMesh`) false true)
          (set `PrimitiveComponent.bGenerateOverlapEvents` false (`self.BottomSpikesCollisionBox`)))
        (:`then_2`
          (`SceneComponent.SetVisibility` (`self.X+SpikesMesh`) false true)
          (set `PrimitiveComponent.bGenerateOverlapEvents` false (`self.X+SpikesCollisionBox`)))
        (:`then_3`
          (`SceneComponent.SetVisibility` (`self.X-SpikesMesh`) false true)
          (set `PrimitiveComponent.bGenerateOverlapEvents` false (`self.X-SpikesCollisionBox`)))
        (:`then_4`
          (`SceneComponent.SetVisibility` (`self.Y+SpikesMesh`) false true)
          (set `PrimitiveComponent.bGenerateOverlapEvents` false (`self.Y+SpikesCollisionBox`)))
        (:`then_5`
          (`SceneComponent.SetVisibility` (`self.Y-SpikesMesh`) false true)
          (set `PrimitiveComponent.bGenerateOverlapEvents` false (`self.Y-SpikesCollisionBox`)))
        (:`then_6`
          (`GameplayStatics.PlaySoundAtLocation` "/Game/SFX/SwordSwipe.SwordSwipe" (`self.K2_GetActorLocation`) (struct) (`self.SwordSwipeVolume`) 1.0 0.0 "/Game/SFX/NaturalSoundAttenuation.NaturalSoundAttenuation" "/Game/Music/StandardSoundConcurrency.StandardSoundConcurrency")
          (set `self.SwordSwipeVolume` 1.0))))))

(fn `ShowOrHideSpikes`
  (bind _topspikes (`self.TopSpikes`))
  (bind _bottomspikes (`self.BottomSpikes`))
  (bind _x_spikes (`self.X+Spikes`))
  (bind _x_spikes_2 (`self.X-Spikes`))
  (bind _y_spikes (`self.Y+Spikes`))
  (bind _y_spikes_2 (`self.Y-Spikes`))
  (if (`self.IsEnable`)
    (`|ExecutionSequence`
      (:`then_0`
        (`SceneComponent.SetVisibility` (`self.TopSpikesMesh`) _topspikes true)
        (set `PrimitiveComponent.bGenerateOverlapEvents` _topspikes (`self.TopSpikesCollisionBox`)))
      (:`then_1`
        (`SceneComponent.SetVisibility` (`self.BottomSpikesMesh`) _bottomspikes true)
        (set `PrimitiveComponent.bGenerateOverlapEvents` _bottomspikes (`self.BottomSpikesCollisionBox`)))
      (:`then_2`
        (`SceneComponent.SetVisibility` (`self.X+SpikesMesh`) _x_spikes true)
        (set `PrimitiveComponent.bGenerateOverlapEvents` _x_spikes (`self.X+SpikesCollisionBox`)))
      (:`then_3`
        (`SceneComponent.SetVisibility` (`self.X-SpikesMesh`) _x_spikes_2 true)
        (set `PrimitiveComponent.bGenerateOverlapEvents` _x_spikes_2 (`self.X-SpikesCollisionBox`)))
      (:`then_4`
        (`SceneComponent.SetVisibility` (`self.Y+SpikesMesh`) _y_spikes true)
        (set `PrimitiveComponent.bGenerateOverlapEvents` _y_spikes (`self.Y+SpikesCollisionBox`)))
      (:`then_5`
        (`SceneComponent.SetVisibility` (`self.Y-SpikesMesh`) _y_spikes_2 true)
        (set `PrimitiveComponent.bGenerateOverlapEvents` _y_spikes_2 (`self.Y-SpikesCollisionBox`)))
      (:`then_6`
        (`GameplayStatics.PlaySoundAtLocation` "/Game/SFX/SwordSwipe.SwordSwipe" (`self.K2_GetActorLocation`) (struct) (`self.SwordSwipeVolume`) 1.0 0.0 "/Game/SFX/NaturalSoundAttenuation.NaturalSoundAttenuation" :!label _label)
        (set `self.SwordSwipeVolume` 1.0)))
    (else
      (`|ExecutionSequence`
        (:`then_0`
          (`SceneComponent.SetVisibility` (`self.TopSpikesMesh`) false true)
          (set `PrimitiveComponent.bGenerateOverlapEvents` false (`self.TopSpikesCollisionBox`)))
        (:`then_1`
          (`SceneComponent.SetVisibility` (`self.BottomSpikesMesh`) false true)
          (set `PrimitiveComponent.bGenerateOverlapEvents` false (`self.BottomSpikesCollisionBox`)))
        (:`then_2`
          (`SceneComponent.SetVisibility` (`self.X+SpikesMesh`) false true)
          (set `PrimitiveComponent.bGenerateOverlapEvents` false (`self.X+SpikesCollisionBox`)))
        (:`then_3`
          (`SceneComponent.SetVisibility` (`self.X-SpikesMesh`) false true)
          (set `PrimitiveComponent.bGenerateOverlapEvents` false (`self.X-SpikesCollisionBox`)))
        (:`then_4`
          (`SceneComponent.SetVisibility` (`self.Y+SpikesMesh`) false true)
          (set `PrimitiveComponent.bGenerateOverlapEvents` false (`self.Y+SpikesCollisionBox`)))
        (:`then_5`
          (`SceneComponent.SetVisibility` (`self.Y-SpikesMesh`) false true)
          (set `PrimitiveComponent.bGenerateOverlapEvents` false (`self.Y-SpikesCollisionBox`)))
        (:`then_6`
          (goto _label))))))

(fn `UserConstructionScript`
  (`parent.UserConstructionScript`)
  (`self.ShowOrHideSpikes`))