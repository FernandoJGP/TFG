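; MovableBlock is a level puzzle Blueprint representing a block that a parent class moves.
; The construction script registers the Block component as ObjectToMove and applies the configurable Material to it.
; BeginPlay and Enable defer to the parent, while Disable calls the parent only when CanContinueDisabling is true.
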(event `self.ReceiveBeginPlay`
  (`parent.ReceiveBeginPlay`))

(event `self.Enable`
  (`parent.Enable`))

(event `self.Disable`
  (if (`self.CanContinueDisabling`)
    (`parent.Disable`)))

(fn `UserConstructionScript`
  (set `self.ObjectToMove` (`self.Block`))
  (`PrimitiveComponent.SetMaterial` (`self.Block`) 0 (`self.Material`)))