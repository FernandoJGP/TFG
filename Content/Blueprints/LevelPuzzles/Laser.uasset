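; Laser hazard for level puzzles that kills the player's MainCharacter on overlap while enabled, unless Blink is active.
; Extends the parent's Enable and Disable to toggle the laser mesh and its buzz audio, hiding and silencing only when CanContinueDisabling allows it.
; The construction script assigns the mesh as the parent's ObjectToMove and configures the buzz sound with natural-sound attenuation.
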(event `self.Enable`
  (`parent.Enable`)
  (`SceneComponent.SetVisibility` (`self.LaserMesh`) true true)
  (`AudioComponent.Play` (`self.LaserAudio`) 0.0))

(event `self.Disable`
  (`parent.Disable`)
  (if (`self.CanContinueDisabling`)
    (`SceneComponent.SetVisibility` (`self.LaserMesh`) false true)
    (`AudioComponent.Stop` (`self.LaserAudio`))))

(event `self.ReceiveActorBeginOverlap`
  (params (OtherActor :type "Actor Object Reference"))
  (bind _returnvalue (`GameplayStatics.GetPlayerPawn` 0))
  (if (== OtherActor _returnvalue)
    (if (`self.IsEnable`)
      (bind _asmain_character (cast `MainCharacter` _returnvalue))
      (if (not (`MainCharacter.bBlinkIsActive` _asmain_character))
        (`MainCharacter.OnDeath` _asmain_character)))))

(fn `UserConstructionScript`
  (set `self.ObjectToMove` (`self.LaserMesh`))
  (`AudioComponent.SetSound` (`self.LaserAudio`) "/Game/SFX/Buzz.Buzz")
  (`AudioComponent.AdjustAttenuation` (`self.LaserAudio`) (make `SoundAttenuationSettings` true true false false false false 0.0 0.0 "SPATIALIZATION_Default" null 3000.0 6000.0 20000.0 20000.0 30.0 60.0 1.0 1.0 1.0 1.0 1.0 1.0 "ECC_Visibility" 20000.0 1.0 0.1 null null 0.3 0.95 400.0 4000.0 "NaturalSound")))