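; A level puzzle display that shows progress toward an objective as "Current/Objective" text on a background panel.
; UpdateText rewrites the TextRender string and swaps the background material to metallic green once Current reaches or exceeds Objective, otherwise metallic red.
; The construction script applies TextSize to the text and calls UpdateText.
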(event `UpdateText`
  (`TextRenderComponent.K2_SetText` (`self.TextRender`) (`KismetTextLibrary.Conv_StringToText` (`KismetStringLibrary.Concat_StrStr` (`KismetStringLibrary.Concat_StrStr` (`KismetStringLibrary.Conv_DoubleToString` (`self.Current`)) " / ") (`KismetStringLibrary.Conv_DoubleToString` (`self.Objective`)))))
  (if (>= (`self.Current`) (`self.Objective`))
    (`PrimitiveComponent.SetMaterial` (`self.Background`) 0 "/Game/Blueprints/LevelPuzzles/Materials/MetalicGreen.MetalicGreen")
    (else
      (`PrimitiveComponent.SetMaterial` (`self.Background`) 0 "/Game/Blueprints/LevelPuzzles/Materials/MetalicRed.MetalicRed"))))

(fn `UserConstructionScript`
  (`TextRenderComponent.SetWorldSize` (`self.TextRender`) (`self.TextSize`))
  (`self.UpdateText`))