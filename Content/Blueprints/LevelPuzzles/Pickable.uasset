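; Puzzle pickup actor whose physics-simulated mesh the player can pick up and drop with the Action input while overlapping it.
; A gate opened on overlap and a busy flag guard input.
; Pickup disables physics, eases the mesh to the character's PickupSocket and attaches it, unless another "pickup"-tagged actor is attached.
; Drop detaches it, moves it using PickupPlacementSocket and re-enables physics.
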(event `self.ReceiveBeginPlay`
  (set `self.InitialWorldPosition` (`self.K2_GetActorLocation`))
  (set `self.InitialWorldRotation` (`self.K2_GetActorRotation`))
  (`self.EnablePhysics`))

(event `InputAction|Action`
  (params (Key :type "Key Structure"))
  (:`Pressed`
    (`/Engine/EditorBlueprintResources/StandardMacros.Gate` true :!label _label
      (:`Exit`
        (if (not (`self.IsBusy`))
          (set `self.IsBusy` true)
          (`GameplayStatics.PlaySoundAtLocation` "/Game/SFX/Click.Click" (`self.K2_GetActorLocation`) (struct) 1.0 1.0 0.0 "/Game/SFX/NaturalSoundAttenuation.NaturalSoundAttenuation")
          (if (`self.IsPicked`)
            (`SceneComponent.K2_DetachFromComponent` (`self.PickupMesh`) "KeepRelative" "KeepRelative" "KeepRelative" true)
            (bind _asmain_character (cast `MainCharacter` (`GameplayStatics.GetPlayerPawn` 0)))
            (`KismetSystemLibrary.MoveComponentTo` (`self.PickupMesh`) (- (`SceneComponent.GetSocketLocation` (`Character.Mesh` _asmain_character) "PickupPlacementSocket") (`SceneComponent.K2_GetComponentLocation` (`self.PickupMesh`))) (struct) true true 0.0)
            (`self.EnablePhysics`)
            (set `self.IsPicked` false)
            (set `self.IsBusy` false)
            (else
              (set `self.PlayerHasPickupAttached` false)
              (for _array_element (`self.GetAttachedActors` (`GameplayStatics.GetPlayerPawn` 0))
                (if (`self.ActorHasTag` _array_element "pickup")
                  (set `self.PlayerHasPickupAttached` true)))
              (if (`self.PlayerHasPickupAttached`)
                (set `self.IsBusy` false)
                (else
                  (`self.DisablePhysics`)
                  (bind _asmain_character_2 (cast `MainCharacter` (`GameplayStatics.GetPlayerPawn` 0)))
                  (bind _mesh (`Character.Mesh` _asmain_character_2))
                  (`KismetSystemLibrary.MoveComponentTo` (`self.PickupMesh`) (`SceneComponent.GetSocketLocation` _mesh "PickupSocket") (`SceneComponent.GetSocketRotation` _mesh "PickupSocket") true true 0.25)
                  (`KismetSystemLibrary.MoveComponentTo` (`self.PickupMesh`) (0.0 0.0 0.0) (struct) false false 0.0)
                  (`SceneComponent.K2_AttachToComponent` (`self.PickupMesh`) _mesh "PickupSocket" "KeepRelative" "KeepRelative" "KeepRelative" false)
                  (set `self.IsPicked` true)
                  (set `self.IsBusy` false))))))))))

(event `self.ReceiveActorBeginOverlap`
  (params (OtherActor :type "Actor Object Reference"))
  (if (== OtherActor (`GameplayStatics.GetPlayerPawn` 0))
    (`self.EnableInput` (`GameplayStatics.GetPlayerController` 0))
    (goto _label :!via `Open`)))

(event `self.ReceiveActorEndOverlap`
  (params (OtherActor :type "Actor Object Reference"))
  (if (== OtherActor (`GameplayStatics.GetPlayerPawn` 0))
    (`self.DisableInput` (`GameplayStatics.GetPlayerController` 0))
    (goto _label :!via `Close`)))

(event `DisablePhysics`
  (`PrimitiveComponent.SetSimulatePhysics` (`self.PickupMesh`) false)
  (`PrimitiveComponent.SetCollisionEnabled` (`self.PickupMesh`) "NoCollision"))

(event `EnablePhysics`
  (`PrimitiveComponent.SetCollisionEnabled` (`self.PickupMesh`) "PhysicsOnly")
  (`PrimitiveComponent.SetSimulatePhysics` (`self.PickupMesh`) true))

(fn `UserConstructionScript`)