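; GoldenSlidingDoor is a level puzzle door that responds only to a powered player.
; On overlap by the player pawn it casts to MainCharacter and calls Enable if IsPowered is set and the door is not already enabled.
; When the player leaves the overlap it calls Disable if enabled, whatever the powered state.
; Enable, Disable and the IsEnable flag are used here but not defined in this graph.
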(event `self.ReceiveActorBeginOverlap`
  (params (OtherActor :type "Actor Object Reference"))
  (bind _returnvalue (`GameplayStatics.GetPlayerPawn` 0))
  (if (== OtherActor _returnvalue)
    (bind _asmain_character (cast `MainCharacter` _returnvalue))
    (if (`MainCharacter.bIsPowered` _asmain_character)
      (if (not (`self.IsEnable`))
        (`self.Enable`)))))

(event `self.ReceiveActorEndOverlap`
  (params (OtherActor :type "Actor Object Reference"))
  (if (== OtherActor (`GameplayStatics.GetPlayerPawn` 0))
    (if (`self.IsEnable`)
      (`self.Disable`))))

(fn `UserConstructionScript`)