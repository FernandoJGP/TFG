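; Puzzle object that slides a component when enabled or disabled, extending a parent's Enable and Disable events.
; Enable either starts an endless back-and-forth loop with a delay at each end or moves once to a configured relative location.
; Disable moves it back to the default zero offset if allowed.
; MoveComponentTo drives timed moves, with pulling audio made audible by volume multiplier only during motion.
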(event `self.ReceiveBeginPlay`
  (`parent.ReceiveBeginPlay`)
  (if (not (`self.FloatingSound`))
    (`AudioComponent.SetSound` (`self.FloatingSoundAudio`) null)))

(event `self.Enable`
  (`parent.Enable`)
  (if (`self.InfiniteMoveLoopAfterEnable`)
    (`self.MoveLoop`)
    (else
      (`self.MoveToEnableLocation`))))

(event `self.Disable`
  (`parent.Disable`)
  (if (`self.CanBeDisabledAfterEnabled`)
    (`self.MoveToDisableLocation`)))

(event `MoveLoop`
  (if (`self.PullingSound`) :!label _label
    (`AudioComponent.SetVolumeMultiplier` (`self.PullingSoundAudio`) 1.0))
  (`KismetSystemLibrary.MoveComponentTo` (`self.ObjectToMove`) (`self.RelativeLocationToMove`) (struct) false false (`self.TimeToReachLocation`))
  (`AudioComponent.SetVolumeMultiplier` (`self.PullingSoundAudio`) 0.0)
  (`KismetSystemLibrary.Delay` (`self.DelayBeforeToggle`))
  (if (`self.PullingSound`)
    (`AudioComponent.SetVolumeMultiplier` (`self.PullingSoundAudio`) 1.0))
  (`KismetSystemLibrary.MoveComponentTo` (`self.ObjectToMove`) (0.0 0.0 0.0) (struct) false false (`self.TimeToReachLocation`))
  (`AudioComponent.SetVolumeMultiplier` (`self.PullingSoundAudio`) 0.0)
  (`KismetSystemLibrary.Delay` (`self.DelayBeforeToggle`))
  (goto _label))

(event `MoveToEnableLocation`
  (if (`self.PullingSound`)
    (`AudioComponent.SetVolumeMultiplier` (`self.PullingSoundAudio`) 1.0))
  (`KismetSystemLibrary.MoveComponentTo` (`self.ObjectToMove`) (`self.RelativeLocationToMove`) (struct) false false (`self.TimeToReachLocation`))
  (`AudioComponent.SetVolumeMultiplier` (`self.PullingSoundAudio`) 0.0))

(event `MoveToDisableLocation`
  (if (`self.PullingSound`)
    (`AudioComponent.SetVolumeMultiplier` (`self.PullingSoundAudio`) 1.0))
  (`KismetSystemLibrary.MoveComponentTo` (`self.ObjectToMove`) (0.0 0.0 0.0) (struct) false false (`self.TimeToReachLocation`))
  (`AudioComponent.SetVolumeMultiplier` (`self.PullingSoundAudio`) 0.0))

(fn `UserConstructionScript`)