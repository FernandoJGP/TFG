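; Activatable is a base Blueprint for level puzzle objects that can be enabled, disabled or toggled.
; BeginPlay applies the initial IsEnable state through Enable or Disable, and Toggle switches between the two.
; Enable records that the object has been enabled at least once, after which Disable only succeeds if CanBeDisabledAfterEnabled allows it.
; Disable reports whether it went through via the CanContinueDisabling flag.
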(event `self.ReceiveBeginPlay`
  (if (`self.IsEnable`)
    (`self.Enable`)
    (else
      (`self.Disable`))))

(event `Enable`
  (set `self.IsEnable` true)
  (set `self.WasEnableAtLeastOneTime` true))

(event `Disable`
  (if (or (not (`self.WasEnableAtLeastOneTime`)) (`self.CanBeDisabledAfterEnabled`))
    (set `self.CanContinueDisabling` true)
    (set `self.IsEnable` false)
    (else
      (set `self.CanContinueDisabling` false))))

(event `Toggle`
  (if (`self.IsEnable`)
    (`self.Disable`)
    (else
      (`self.Enable`))))

(fn `UserConstructionScript`)