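; Collectible pickup with a spinning katana that the player collects on overlap, persisting across sessions.
; BeginPlay destroys it if its ID is already marked in the achievements save.
; Overlap destroys it, plays sounds, saves the flag, then counts collected items and prints progress in English or Spanish, based on saved settings.
; Milestone counts print an achievement message and show its name and image on the HUD overlay.
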(event `self.ReceiveBeginPlay`
  (bind _returnvalue (`GameplayStatics.DoesSaveGameExist` (`self.AchievementsSlotName`)))
  (if _returnvalue
    (bind _returnvalue_2 (`GameplayStatics.LoadGameFromSlot` (`self.AchievementsSlotName`)))
    (bind _output_get (set `self.AchievementsReference` _returnvalue_2))
    (bind _asachievements_save_game (cast `/Game/Blueprints/SaveGames/AchievementsSaveGame` _output_get))
    (if (`|GetArrayItem` (`/Game/Blueprints/SaveGames/AchievementsSaveGame.CollectedCollectibles` _asachievements_save_game) (`self.ID`))
      (`SceneComponent.SetVisibility` (`self.Scene`) false true)
      (`self.K2_DestroyActor`))))

(event `self.ReceiveActorBeginOverlap`
  (params (OtherActor :type "Actor Object Reference"))
  (if (== OtherActor (`GameplayStatics.GetPlayerPawn` 0))
    (`self.K2_DestroyActor`)
    (`GameplayStatics.PlaySoundAtLocation` null (`self.K2_GetActorLocation`))
    (bind _returnvalue (`GameplayStatics.DoesSaveGameExist` (`self.AchievementsSlotName`)))
    (if _returnvalue
      (bind _returnvalue_2 (`GameplayStatics.LoadGameFromSlot` (`self.AchievementsSlotName`)))
      (set `self.AchievementsReference` _returnvalue_2)
      (else
        (bind _returnvalue_3 (`GameplayStatics.CreateSaveGameObject` "/Game/Blueprints/SaveGames/AchievementsSaveGame.AchievementsSaveGame_C"))
        (set `self.AchievementsReference` _returnvalue_3)))
    (bind _asachievements_save_game (cast `/Game/Blueprints/SaveGames/AchievementsSaveGame` (`self.AchievementsReference`)))
    (`KismetArrayLibrary.Array_Set` (`/Game/Blueprints/SaveGames/AchievementsSaveGame.CollectedCollectibles` _asachievements_save_game) (`self.ID`) true)
    (`GameplayStatics.SaveGameToSlot` (`self.AchievementsReference`) (`self.AchievementsSlotName`))
    (`self.ShowCollectibleAchievementsProgress`)
    (`GameplayStatics.PlaySoundAtLocation` "/Game/SFX/SwordSwipe.SwordSwipe" (`self.K2_GetActorLocation`))))

(event `self.ReceiveTick`
  (params (DeltaSeconds :type "Float (single-precision)"))
  (bind _innerrotationspeed (`self.InnerRotationSpeed`))
  ;[1 1 1] Rotation
  (`SceneComponent.K2_AddLocalRotation` (`self.Katana`) (* (`KismetMathLibrary.MakeRotator` 0.0 0.0 (`self.RotationSpeed`)) DeltaSeconds) false false)
  (`SceneComponent.K2_AddLocalRotation` (`self.Scene2`) (* (`KismetMathLibrary.MakeRotator` _innerrotationspeed _innerrotationspeed _innerrotationspeed) DeltaSeconds) false false))

(fn `ShowCollectibleAchievementsProgress`
  (bind _asachievements_save_game (cast `/Game/Blueprints/SaveGames/AchievementsSaveGame` (`self.AchievementsReference`)))
  (for _array_element (`/Game/Blueprints/SaveGames/AchievementsSaveGame.CollectedCollectibles` _asachievements_save_game)
    (if _array_element
      (`/Engine/EditorBlueprintResources/StandardMacros.IncrementInt` (`self.NumberOfCollectedCollectibles`))))
  (bind _returnvalue (`GameplayStatics.DoesSaveGameExist` (`self.SettingsSlotName`)))
  (if _returnvalue
    (bind _returnvalue_2 (`GameplayStatics.LoadGameFromSlot` (`self.SettingsSlotName`)))
    (bind _assettings_save_game (cast `/Game/Blueprints/SaveGames/SettingsSaveGame` _returnvalue_2))
    (bind _output_get (set `self.Language` (`/Game/Blueprints/SaveGames/SettingsSaveGame.Language` _assettings_save_game)))
    (switch `string` _output_get
      (:`Default`
        (set `self.StringToPrint` "Collectible progress: " :!label _label))
      (:`en`
        (goto _label))
      (:`es`
        (set `self.StringToPrint` "Progreso en coleccionables: ")))
    (else
      (goto _label)))
  (bind _output_get_2 (set `self.StringToPrint` (`KismetStringLibrary.Concat_StrStr` (`self.StringToPrint`) (`KismetStringLibrary.Conv_IntToString` (`self.NumberOfCollectedCollectibles`)))))
  (bind _output_get_3 (set `self.StringToPrint` (`KismetStringLibrary.Concat_StrStr` _output_get_2 "/")))
  (bind _output_get_4 (set `self.StringToPrint` (`KismetStringLibrary.Concat_StrStr` _output_get_3 (`KismetStringLibrary.Conv_IntToString` (`self.TotalNumberOfCollectibles`)))))
  (`KismetSystemLibrary.PrintString` _output_get_4 true true (struct :`R` 0.991102 :`G` 0.082283 :`A` 1.0) 5.0)
  (`self.ShowNewCollectibleAchievements`)
  (return))

(fn `ShowNewCollectibleAchievements`
  (switch `string` (`self.Language`)
    (:`Default`
      (set `self.StringToPrint` "Achievement unlocked!: " :!label _label))
    (:`en`
      (goto _label))
    (:`es`
      (set `self.StringToPrint` "¡Logro desbloqueado!: ")))
  (switch `int` (`self.NumberOfCollectedCollectibles`)
    (:`1`
      (switch `string` (`self.Language`)
        (:`Default`
          (set `self.Achievement` "Collectibles 1" :!label _label_2))
        (:`en`
          (goto _label_2))
        (:`es`
          (set `self.Achievement` "Coleccionables 1")))
      (set `self.AchievementImage` "/Game/Blueprints/HUDs/UserHUD/Textures/Achievements/achievement-collectible-1.achievement-collectible-1"))
    (:`5`
      (switch `string` (`self.Language`)
        (:`Default`
          (set `self.Achievement` "Collectibles 5" :!label _label_3))
        (:`en`
          (goto _label_3))
        (:`es`
          (set `self.Achievement` "Coleccionables 5")))
      (set `self.AchievementImage` "/Game/Blueprints/HUDs/UserHUD/Textures/Achievements/achievement-collectible-5.achievement-collectible-5"))
    (:`10`
      (switch `string` (`self.Language`)
        (:`Default`
          (set `self.Achievement` "Collectibles 10" :!label _label_4))
        (:`en`
          (goto _label_4))
        (:`es`
          (set `self.Achievement` "Coleccionables 10")))
      (set `self.AchievementImage` "/Game/Blueprints/HUDs/UserHUD/Textures/Achievements/achievement-collectible-10.achievement-collectible-10"))
    (:`15`
      (switch `string` (`self.Language`)
        (:`Default`
          (set `self.Achievement` "Collectibles 50%" :!label _label_5))
        (:`en`
          (goto _label_5))
        (:`es`
          (set `self.Achievement` "Coleccionables 50%")))
      (set `self.AchievementImage` "/Game/Blueprints/HUDs/UserHUD/Textures/Achievements/achievement-collectible-50x100.achievement-collectible-50x100"))
    (:`30`
      (switch `string` (`self.Language`)
        (:`Default`
          (set `self.Achievement` "Collectibles 100%" :!label _label_6))
        (:`en`
          (goto _label_6))
        (:`es`
          (set `self.Achievement` "Coleccionables 100%")))
      (set `self.AchievementImage` "/Game/Blueprints/HUDs/UserHUD/Textures/Achievements/achievement-collectible-100x100.achievement-collectible-100x100")))
  (set `self.StringToPrint` (`KismetStringLibrary.Concat_StrStr` (`self.StringToPrint`) (`self.Achievement`)))
  (`KismetSystemLibrary.PrintString` (`self.StringToPrint`) true true (struct :`R` 0.991102 :`G` 0.082283 :`A` 1.0) 10.0)
  (bind _foundwidgets (`WidgetBlueprintLibrary.GetAllWidgetsOfClass` "/Game/Blueprints/HUDs/UserHUD/UserHUDWidget.UserHUDWidget_C"))
  (bind _output (`|GetArrayItem` _foundwidgets))
  (set `/Game/Blueprints/HUDs/UserHUD/UserHUDWidget.Achievement` (`self.Achievement`) _output)
  (set `/Game/Blueprints/HUDs/UserHUD/UserHUDWidget.AchievementImage` (`self.AchievementImage`) _output)
  (`/Game/Blueprints/HUDs/UserHUD/UserHUDWidget.ShowAchievementOverlay` _output)
  (return))

(fn `UserConstructionScript`)